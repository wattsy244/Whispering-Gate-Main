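; BP_SlidingDoor is a door that slides open while the player character is inside its trigger Box and closes when they leave.
; Box overlap events play and reverse the OpenClose timeline, ignoring other actors.
; Its DoorTrack value drives Lerps on four cube panels: one pair parts sideways along X, while a second pair, offset in Y, parts vertically along Z.
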(event `self.Box.OnComponentBeginOverlap`
  (params (OverlappedComponent :type "PrimitiveComponent Object Reference") (OtherActor :type "Actor Object Reference") (OtherComp :type "PrimitiveComponent Object Reference") (OtherBodyIndex :type Integer) (bFromSweep :type Boolean) (SweepResult :type "HitResult Structure (by ref)"))
  (if (== OtherActor (`GameplayStatics.GetPlayerCharacter` 0))
    (bind (_direction _door_track) (`Timeline|Open/Close` :!label _label)
      (:`Update`
        (`|ExecutionSequence`
          (:`then_0`
            (`SceneComponent.K2_SetRelativeLocation` (`self.Cube-Left`) (`KismetMathLibrary.MakeVector` (`KismetMathLibrary.Lerp` -50.0 -200.0 _door_track) 0.0 100.0) false false))
          (:`then_1`
            (`SceneComponent.K2_SetRelativeLocation` (`self.Cube-Right`) (`KismetMathLibrary.MakeVector` (`KismetMathLibrary.Lerp` 50.0 200.0 _door_track) 0.0 100.0) false false))
          (:`then_2`
            (`SceneComponent.K2_SetRelativeLocation` (`self.Cube-up1`) (`KismetMathLibrary.MakeVector` 0.0 -20.0 (`KismetMathLibrary.Lerp` 150.0 300.0 _door_track)) false false))
          (:`then_3`
            (`SceneComponent.K2_SetRelativeLocation` (`self.Cube-down1`) (`KismetMathLibrary.MakeVector` 0.0 -20.0 (`KismetMathLibrary.Lerp` 50.0 -100.0 _door_track)) false false)))))))

(event `self.Box.OnComponentEndOverlap`
  (params (OverlappedComponent :type "PrimitiveComponent Object Reference") (OtherActor :type "Actor Object Reference") (OtherComp :type "PrimitiveComponent Object Reference") (OtherBodyIndex :type Integer))
  (if (== OtherActor (`GameplayStatics.GetPlayerCharacter` 0))
    (goto _label :!via `Reverse`)))

(fn `UserConstructionScript`)