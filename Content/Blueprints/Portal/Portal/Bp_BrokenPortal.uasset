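; Broken portal actor that collects built parts and replaces itself with a working Bp_Portal once complete.
; BeginPlay restores the built count from saved game data through the GameInstance.
; Each Build event records the part index, increments the count, saves player and parts data, and spawns the portal when the target is reached.
; Its box overlap passes the teleport level name to any Bp_Portal it touches.
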(event `self.ReceiveBeginPlay`
  (bind _savegamedata (message `/Game/Blueprints/Checkpoints/BPI_SaveGame.GetGameData` (`GameplayStatics.GetGameInstance`)))
  (set `self.Total parts` (`/Game/Blueprints/Checkpoints/BP_Checkpoint.BuiltAmount` _savegamedata)))

(event `/Game/Blueprints/Portal/Portal/BPI_Build.Build`
  (params (PartIndex :type Integer))
  ; sets parts/ saves player data
  (`KismetArrayLibrary.Array_Add` (`self.PartBuilt`) PartIndex)
  (bind _output_get (set `self.CurrentParts` 1.0))
  (set `self.Total parts` (+ (`self.Total parts`) _output_get))
  (bind _asbp_first_person_character (cast `/Game/FirstPerson/Blueprints/BP_FirstPersonCharacter` (stale `self.Box.OnComponentBeginOverlap` OtherActor)))
  (bind _playersave (`/Game/FirstPerson/Blueprints/BP_FirstPersonCharacter.GetPlayerData` _asbp_first_person_character))
  (message `/Game/Blueprints/Checkpoints/BPI_SaveGame.SavePlayerData` (`GameplayStatics.GetGameInstance`) _playersave false)
  ; saves parts
  (message `/Game/Blueprints/Checkpoints/BPI_SaveGame.SaveParts` (`GameplayStatics.GetGameInstance`) true)
  (`GameplayStatics.PlaySound2D` "/Game/FPWeapon/Audio/FirstPersonTemplateWeaponFire02.FirstPersonTemplateWeaponFire02" 1.0 1.0 0.0 null null)
  ; checks all parts are added
  (`KismetSystemLibrary.PrintString` (`KismetStringLibrary.Conv_DoubleToString` (`self.Total parts`)))
  (if (== (`self.Total parts`) (`self.BuildAmount`))
    ; Spawns portal
    (`self.K2_DestroyActor`)
    (`|SpawnActorFromClass` "/Game/Blueprints/Portal/Portal/Bp_Portal.Bp_Portal_C" (`KismetMathLibrary.Conv_VectorToTransform` (`self.K2_GetActorLocation`)) "Undefined" "MultiplyWithRoot" null (`self.Level`) null)
    (`KismetSystemLibrary.PrintString` "portal spawn")))

(event `self.Box.OnComponentBeginOverlap`
  (params (OverlappedComponent :type "PrimitiveComponent Object Reference") (OtherActor :type "Actor Object Reference") (OtherComp :type "PrimitiveComponent Object Reference") (OtherBodyIndex :type Integer) (bFromSweep :type Boolean) (SweepResult :type "HitResult Structure (by ref)"))
  ; sets parts/ saves player data
  (bind _asbp_portal (cast `/Game/Blueprints/Portal/Portal/Bp_Portal` OtherActor))
  (set `/Game/Blueprints/Portal/Portal/Bp_Portal.LevelName` (`self.TeleportLocation`) _asbp_portal))

(fn `UserConstructionScript`)