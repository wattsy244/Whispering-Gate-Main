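; Collectible portal part actor that the player picks up through an Interact event.
; On BeginPlay it destroys itself if its Index is already in the GameInstance save data's PartsIndex.
; Interact prints a debug message and destroys the actor on the next tick, without writing to the save data itself.
; The construction script applies the PortalPartMesh variable to the mesh component.
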(event `self.ReceiveBeginPlay`
  (bind _asbp_game_instance (cast `/Game/Blueprints/Checkpoints/BP_GameInstance` (`GameplayStatics.GetGameInstance`)))
  (if (`KismetArrayLibrary.Array_Contains` (`/Game/Blueprints/Checkpoints/BP_Checkpoint.PartsIndex` (`/Game/Blueprints/Checkpoints/BP_GameInstance.SaveData` _asbp_game_instance)) (`self.Index`))
    (`self.K2_DestroyActor`)))

(event `/Game/Blueprints/Portal/Portal/BPI_Interact.Interact`
  (`KismetSystemLibrary.PrintString` "Part picked up")
  (`KismetSystemLibrary.DelayUntilNextTick`)
  (`self.K2_DestroyActor`))

(fn `UserConstructionScript`
  (`StaticMeshComponent.SetStaticMesh` (`self.PartMesh`) (`self.PortalPartMesh`)))