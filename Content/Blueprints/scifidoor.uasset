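; A sci-fi door Blueprint that opens when the first-person character enters its trigger box and closes when they leave.
; On BeginPlay it stores the actor location as the closed position.
; Overlap events play a Timeline from the start or reverse it, lerping the static mesh's world location toward a Billboard component that marks the open position.
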(event `self.ReceiveBeginPlay`
  (set `self.Origin` (`self.K2_GetActorLocation`)))

(event `self.Box.OnComponentBeginOverlap`
  (params (OverlappedComponent :type "PrimitiveComponent Object Reference") (OtherActor :type "Actor Object Reference") (OtherComp :type "PrimitiveComponent Object Reference") (OtherBodyIndex :type Integer) (bFromSweep :type Boolean) (SweepResult :type "HitResult Structure (by ref)"))
  (if (== (`GameplayStatics.GetObjectClass` OtherActor) "/Game/FirstPerson/Blueprints/BP_FirstPersonCharacter.BP_FirstPersonCharacter_C")
    (`self.Raise Door`)))

(event `self.Box.OnComponentEndOverlap`
  (params (OverlappedComponent :type "PrimitiveComponent Object Reference") (OtherActor :type "Actor Object Reference") (OtherComp :type "PrimitiveComponent Object Reference") (OtherBodyIndex :type Integer))
  (if (== (`GameplayStatics.GetObjectClass` OtherActor) "/Game/FirstPerson/Blueprints/BP_FirstPersonCharacter.BP_FirstPersonCharacter_C")
    (`self.Lower Door`)))

(event `Raise Door`
  (bind (_direction _newtrack_0) (`Timeline|Timeline` :!via `PlayFromStart` :!label _label)
    (:`Update`
      (`SceneComponent.K2_SetWorldLocation` (`self.StaticMesh`) (`KismetMathLibrary.VLerp` (`self.Origin`) (`SceneComponent.K2_GetComponentLocation` (`self.Billboard`)) _newtrack_0) false false))))

(event `Lower Door`
  (goto _label :!via `Reverse`))

(fn `UserConstructionScript`)