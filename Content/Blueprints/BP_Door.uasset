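; BP_Door is an interactable door with a number pad UI, usable while the first-person character is inside its trigger.
; Overlap enables input and a text prompt; leaving reverses both and clears widgets.
; E or the OpenTheDoor event plays a timeline that drives one door mesh and starts a second timeline for the other.
; L toggles the W_NumberPad widget, switching input mode and cursor visibility.
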(event `Key|E`
  (params (Key :type "Key Structure"))
  ; Doors open
  (:`Pressed`
    (`Timeline|Timeline` :!label _label
      (:`Update`
        (`SceneComponent.K2_SetRelativeLocation` (`self.door_up_white`) (0.0 0.0 0.0) false false)
        (`Timeline|Timeline_0`
          (:`Update`
            (`SceneComponent.K2_SetRelativeLocation` (`self.door_up_white1`) (0.0 0.0 0.0) false false)))))))

(event `Open The Door`
  ; Doors open
  (goto _label))

(event `self.r.OnComponentBeginOverlap`
  (params (OverlappedComponent :type "PrimitiveComponent Object Reference") (OtherActor :type "Actor Object Reference") (OtherComp :type "PrimitiveComponent Object Reference") (OtherBodyIndex :type Integer) (bFromSweep :type Boolean) (SweepResult :type "HitResult Structure (by ref)"))
  (cast `/Game/FirstPerson/Blueprints/BP_FirstPersonCharacter` OtherActor)
  (`self.EnableInput` (`GameplayStatics.GetPlayerController` 0))
  (`SceneComponent.SetVisibility` (`self.TextRender`) true false))

(event `self.r.OnComponentEndOverlap`
  (params (OverlappedComponent :type "PrimitiveComponent Object Reference") (OtherActor :type "Actor Object Reference") (OtherComp :type "PrimitiveComponent Object Reference") (OtherBodyIndex :type Integer))
  (bind _returnvalue (`GameplayStatics.GetPlayerController` 0))
  (cast `/Game/FirstPerson/Blueprints/BP_FirstPersonCharacter` OtherActor)
  (`self.DisableInput` null)
  (`SceneComponent.SetVisibility` (`self.TextRender`) false false)
  (`WidgetLayoutLibrary.RemoveAllWidgets` :!label _label_2)
  (`WidgetBlueprintLibrary.SetInputMode_GameOnly` _returnvalue)
  (set `PlayerController.bShowMouseCursor` false _returnvalue))

(event `Key|L`
  (params (Key :type "Key Structure"))
  (bind _returnvalue (`GameplayStatics.GetPlayerController` 0))
  (:`Pressed`
    (`/Engine/EditorBlueprintResources/StandardMacros.FlipFlop`
      (:`A`
        (bind _returnvalue_2 (`|CreateWidget` "/Game/Blueprints/W_NumberPad.W_NumberPad_C"))
        (`UserWidget.AddToViewport` _returnvalue_2 0)
        (`WidgetBlueprintLibrary.SetInputMode_GameAndUIEx` _returnvalue _returnvalue_2)
        (set `PlayerController.bShowMouseCursor` true _returnvalue))
      (:`B`
        (goto _label_2)))))

(fn `UserConstructionScript`)