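; BP_Cam is a camera actor that detects the first-person player through a PawnSensing component and damages them after repeated sightings.
; While IsOn, which is set at BeginPlay, each sighting of BP_FirstPersonCharacter adds a fixed increment to SeenFor.
; Once SeenFor reaches TotalTime, it applies damage and stores the returned damage value back into SeenFor instead of resetting it to zero.
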(event `self.ReceiveBeginPlay`
  (set `self.Is_On` true))

(event `self.PawnSensing.OnSeePawn`
  (params (Pawn :type "Pawn Object Reference"))
  ; Detect player
  (if (`self.Is_On`)
    (bind _asbp_first_person_character (cast `/Game/FirstPerson/Blueprints/BP_FirstPersonCharacter` Pawn))
    (bind _output_get (set `self.CurrentTime` 1.0))
    (bind _output_get_2 (set `self.SeenFor` (+ _output_get (`self.SeenFor`))))
    (if (>= _output_get_2 (`self.TotalTime`))
      (bind _returnvalue (`GameplayStatics.ApplyDamage` _asbp_first_person_character 33.0))
      (set `self.SeenFor` _returnvalue))))

(fn `UserConstructionScript`)