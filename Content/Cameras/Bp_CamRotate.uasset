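; Rotating surveillance camera actor that sweeps back and forth and damages the player when it spots them.
; A Timeline drives absolute yaw from BeginPlay, alternating forward and reverse playback each time it finishes.
; PawnSensing sightings of BP_FirstPersonCharacter increment a cumulative counter, which applies damage and resets upon equalling TotalTime.
; The IsOn flag gates both the sweep and detection.
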(event `self.ReceiveBeginPlay`
  (`self.Rotate`))

(event `Rotate`
  (bind (_returnvalue_roll _returnvalue_pitch) (`KismetMathLibrary.BreakRotator` (`self.K2_GetActorRotation` self)))
  ; Rotates camera
  (if (`self.isOn`)
    (bind (_direction _newtrack_0) (`Timeline|Timeline` :!label _label)
      (:`Update`
        (bind (_returnvalue_roll_2 _returnvalue_pitch_2 _returnvalue_yaw) (`KismetMathLibrary.BreakRotator` (`KismetMathLibrary.MakeRotator` 0.0 0.0 _newtrack_0)))
        (`self.K2_SetActorRotation` (`KismetMathLibrary.MakeRotator` _returnvalue_roll _returnvalue_pitch _returnvalue_yaw)))
      (:`Finished`
        (switch `ETimelineDirection` _direction
          (:`Forward`
            (`self.Reverse`))
          (:`Backward`
            (`self.Rotate`)))))))

(event `Reverse`
  ; Rotates camera
  (if (`self.isOn`)
    (goto _label :!via `Reverse`)))

(event `self.PawnSensing.OnSeePawn`
  (params (Pawn :type "Pawn Object Reference"))
  ; Detects player and deals damage
  (if (`self.isOn`)
    (bind _asbp_first_person_character (cast `/Game/FirstPerson/Blueprints/BP_FirstPersonCharacter` Pawn))
    (bind _output_get (set `self.CurrentTime` 1.0))
    (bind _output_get_2 (set `self.seenFor` (+ _output_get (`self.seenFor`))))
    (if (== _output_get_2 (`self.TotalTime`))
      (`GameplayStatics.ApplyDamage` _asbp_first_person_character 33.0)
      (set `self.seenFor` 0.0))))

(fn `UserConstructionScript`)